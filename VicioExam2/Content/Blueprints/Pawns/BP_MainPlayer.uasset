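; BP_MainPlayer is the player pawn, handling movement, camera look and coin collection.
; An Enhanced Input action moves it relative to control rotation, while legacy MouseX and MouseY axis events drive yaw and pitch.
; On BeginPlay it creates the coin widget, and AddCoin pushes each new total to it.
; Whenever that total is divisible by three, AddCoin spawns a BP_Enemy at random X/Y coordinates within a fixed range.
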(event `EnhancedInput|/Game/Blueprints/Inputs/IA_Moverse`
  (params (ActionValue :type "Vector2D Structure") (ElapsedSeconds :type "Float (double-precision)") (TriggeredSeconds :type "Float (double-precision)") (InputAction :type "InputAction Object Reference" :default "/Game/Blueprints/Inputs/IA_Moverse.IA_Moverse"))
  (bind (_returnvalue_roll _returnvalue_pitch _returnvalue_yaw) (`KismetMathLibrary.BreakRotator` (`self.GetControlRotation`)))
  (bind (_returnvalue_roll_2 _returnvalue_pitch_2 _returnvalue_yaw_2) (`KismetMathLibrary.BreakRotator` (`self.GetControlRotation`)))
  ;[0.6572 1 0.33] Movimiento
  (:`Triggered`
    (`self.AddMovementInput` (`KismetMathLibrary.GetForwardVector` (`KismetMathLibrary.MakeRotator` _returnvalue_roll 0.0 _returnvalue_yaw)) ActionValue_X)
    (`self.AddMovementInput` (`KismetMathLibrary.GetRightVector` (`KismetMathLibrary.MakeRotator` _returnvalue_roll_2 0.0 _returnvalue_yaw_2)) ActionValue_Y)))

(event `InputAxisKey|MouseY`
  (params (AxisValue :type "Float (single-precision)"))
  ;[0.05098 0 0] Camara
  (`self.AddControllerPitchInput` AxisValue))

(event `InputAxisKey|MouseX`
  (params (AxisValue :type "Float (single-precision)"))
  ;[0.05098 0 0] Camara
  (`self.AddControllerYawInput` AxisValue))

(event `self.ReceiveBeginPlay`
  ;[0.05098 0.01673 0] UI Coins
  (bind _returnvalue (`|CreateWidget` "/Game/Blueprints/HUD/WBP_CoinUI.WBP_CoinUI_C"))
  (bind _output_get (set `self.Main UI` _returnvalue))
  (`UserWidget.AddToViewport` _output_get 0)
  (set `/Game/Blueprints/HUD/WBP_CoinUI.COIN` (`self.Coin`) (`self.Main UI`)))

(event `Add Coin`
  (params (`Coin Value` :type Integer))
  (bind (_returnvalue_x _returnvalue_y) (`KismetMathLibrary.BreakVector` (`KismetMathLibrary.MakeVector` (`KismetMathLibrary.RandomFloatInRange` 200.0 2890.0) (`KismetMathLibrary.RandomFloatInRange` 200.0 2890.0) 45.0)))
  ;[0.05098 0.01673 0] UI Coins
  (bind _output_get (set `self.Coin` (+ (`self.Coin`) `Coin Value`)))
  (bind _output_get_2 (set `/Game/Blueprints/HUD/WBP_CoinUI.COIN` _output_get (`self.Main UI`)))
  (if (== (`KismetMathLibrary.FMod` (`KismetMathLibrary.Conv_IntToDouble` _output_get_2) 3.0) 0.0)
    (`|SpawnActorFromClass` "/Game/Blueprints/Pawns/BP_Enemy.BP_Enemy_C" (`KismetMathLibrary.MakeTransform` (`KismetMathLibrary.MakeVector` _returnvalue_x _returnvalue_y)) "Undefined" "MultiplyWithRoot" null null)))

(fn `UserConstructionScript`)