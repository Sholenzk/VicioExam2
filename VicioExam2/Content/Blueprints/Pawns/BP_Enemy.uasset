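; BP_Enemy is an enemy that continuously moves straight toward the first player character.
; Each Tick it offsets its location along the normalized direction to the player, scaled by Velocity and delta time, without sweeping for collision.
; It then sets yaw from a look-at rotation computed from the player to itself, so its forward axis points away from the player.
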(event `self.ReceiveTick`
  (params (DeltaSeconds :type "Float (single-precision)"))
  (bind _returnvalue (`self.K2_GetActorLocation`))
  (bind _returnvalue_2 (`self.K2_GetActorLocation` (`GameplayStatics.GetPlayerCharacter` 0)))
  (bind (_returnvalue_roll _returnvalue_pitch _returnvalue_yaw) (`KismetMathLibrary.BreakRotator` (`KismetMathLibrary.FindLookAtRotation` _returnvalue_2 _returnvalue)))
  ;[0.1823 0 0] Enemy Spawn
  (`self.K2_SetActorLocation` (+ (* (`KismetMathLibrary.Normal` (- _returnvalue_2 _returnvalue)) DeltaSeconds (`self.Velocity`)) _returnvalue))
  (`self.K2_SetActorRotation` (`KismetMathLibrary.MakeRotator` 0.0 0.0 _returnvalue_yaw)))

(fn `UserConstructionScript`)